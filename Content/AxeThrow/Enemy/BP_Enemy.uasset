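; BP_Enemy is an axe-throw game enemy with a health component and a health bar widget.
; On BeginPlay it casts the HealthBar widget to WBP_EnemyHealth and passes itself as that widget's enemy reference.
; Every Tick it polls HealthComponent health and destroys the actor once it reaches zero or below.
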(event `self.ReceiveBeginPlay`
  (bind _aswbp_enemy_health (cast `/Game/UI/WBP_EnemyHealth` (`WidgetComponent.GetWidget` (`self.HealthBar`))))
  (set `/Game/UI/WBP_EnemyHealth.As BP Enemy` self _aswbp_enemy_health))

(event `self.ReceiveTick`
  (params (DeltaSeconds :type "Float (single-precision)"))
  (if (<= (`BaseStatsComponent.Health` (`self.HealthComponent`)) 0.0)
    (`self.K2_DestroyActor`)))

(fn `UserConstructionScript`)