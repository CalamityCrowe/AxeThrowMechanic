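; Player character for the axe-throw mechanic, handling the axe's animations, melee combo, target lock and camera feedback.
; Events trigger equip, throw and catch animations plus camera shake, while a timeline blends the camera in and out of aiming.
; Melee input picks one of four combo montages from the Pickaxe MeleeComponent's attack count, which Tick prints for debugging.
; Q triggers TargetLockOn and the mouse wheel switches targets.
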(event `self.ReceiveBeginPlay`)

(event `self.ShakeCamera`
  (`PlayerCameraManager.StartCameraShake` :`self` (`GameplayStatics.GetPlayerCameraManager` 0) :`ShakeClass` "/Game/AxeThrow/Blueprint/CameraShake.CameraShake_C" :`Scale` 6.0))

(event `self.EquipAnim`
  (if (`|EnumEquality` (`BaseThrowable.AxeState` (`self.Pickaxe`)) "Idle")
    (bind _asaxethrow_abp (cast `/Game/AxeThrow/Animations/Sequences/Test/Axethrow_ABP` (`SkeletalMeshComponent.GetAnimInstance` (`self.Mesh`))))
    (set `/Game/AxeThrow/Animations/Sequences/Test/Axethrow_ABP.PlayEquipAnim` true _asaxethrow_abp)))

(event `Key|Q`
  (params (Key :type "Key Structure"))
  (:`Pressed`
    (`TargetLockOnComponent.TriggerTargetLockOn` (`self.TargetLockOn`))))

(event `self.ThrowMontage`
  (`|PlayMontage` (`self.Mesh`) "/Game/AxeThrow/Animations/Sequences/Test/Quinn_Throw1_Montage.Quinn_Throw1_Montage"))

(event `Key|MouseScrollUp`
  (params (Key :type "Key Structure"))
  (:`Pressed`
    (`TargetLockOnComponent.SwitchTarget` (`self.TargetLockOn`) -1.0)))

(event `self.CatchMontage`
  (`|PlayMontage` (`self.Mesh`) "/Game/AxeThrow/Animations/Sequences/Test/Quinn_Aiming_Montage.Quinn_Aiming_Montage" 2.0))

(event `Key|MouseScrollDown`
  (params (Key :type "Key Structure"))
  (:`Pressed`
    (`TargetLockOnComponent.SwitchTarget` (`self.TargetLockOn`) 1.0)))

(event `EnhancedInput|/Game/Inputs/Actions/IA_Melee`
  (params (ActionValue :type Boolean) (ElapsedSeconds :type "Float (double-precision)") (TriggeredSeconds :type "Float (double-precision)") (InputAction :type "InputAction Object Reference" :default "/Game/Inputs/Actions/IA_Melee.IA_Melee"))
  (:`Started`
    (if (and (`self.isEquipped`) (and (not (`self.isAiming`)) (not (`self.isThrowing`))))
      (if (not (`self.IsAttacking`))
        (`|PlayMontage` (`self.Mesh`) (select `int` (`MeleeAttackComponent.AttackCount` (`BaseThrowable.MeleeComponent` (`self.Pickaxe`))) :`0` "/Game/ARPG_Warrior/Animations/ARPG_Warrior_Anim_UE_Attack_Combo1_Montage.ARPG_Warrior_Anim_UE_Attack_Combo1_Montage" :`1` "/Game/ARPG_Warrior/Animations/ARPG_Warrior_Anim_UE_Attack_Combo2_Montage.ARPG_Warrior_Anim_UE_Attack_Combo2_Montage" :`2` "/Game/ARPG_Warrior/Animations/ARPG_Warrior_Anim_UE_Attack_Combo3_Montage.ARPG_Warrior_Anim_UE_Attack_Combo3_Montage" :`3` "/Game/ARPG_Warrior/Animations/ARPG_Warrior_Anim_UE_Attack_Combo4_Montage.ARPG_Warrior_Anim_UE_Attack_Combo4_Montage" :!type "AnimMontage Object Reference")
          (:`then`
            (set `self.IsAttacking` true)
            (`/Engine/EditorBlueprintResources/StandardMacros.IncrementInt` (`MeleeAttackComponent.AttackCount` (`BaseThrowable.MeleeComponent` (`self.Pickaxe`)))))
          (:`OnCompleted`
            (set `MeleeAttackComponent.AttackCount` 0 (`BaseThrowable.MeleeComponent` (`self.Pickaxe`))))
          (:`OnInterrupted`
            (`KismetSystemLibrary.RetriggerableDelay` 2.5)
            (set `MeleeAttackComponent.bIsAttacking` false (`BaseThrowable.MeleeComponent` (`self.Pickaxe`)))))))))

(event `self.ReceiveTick`
  (params (DeltaSeconds :type "Float (single-precision)"))
  (`KismetSystemLibrary.PrintString` (`KismetStringLibrary.Conv_IntToString` (`MeleeAttackComponent.AttackCount` (`BaseThrowable.MeleeComponent` (`self.Pickaxe`)))) true true (struct :`G` 0.66 :`B` 1.0 :`A` 1.0) 0.2))

(event `self.LerpCamera`
  (bind _camera_lerping (`self.Camera Lerping`))
  (if (`self.isAiming`)
    (`TimelineComponent.SetPlayRate` _camera_lerping 1.4)
    (bind (_direction _alpha) (`Timeline|Camera Lerping` :!label _label)
      (:`Update`
        (`self.LerpCameraAlpha` _alpha)))
    (else
      (`TimelineComponent.SetPlayRate` _camera_lerping 0.9)
      (goto _label :!via `Reverse`))))

(fn `UserConstructionScript`)